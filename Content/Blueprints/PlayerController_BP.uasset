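; Player controller Blueprint that draws a red "cane" line extending from the controlled pawn's viewpoint.
; Each Tick passes the pawn's eye location and rotation to FindCaneEnd, which projects the endpoint along the forward vector by CaneLength.
; The cane is only a debug line drawn with CaneThickness, with no trace or collision check.
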(event `self.ReceiveTick`
  (params (DeltaSeconds :type "Float (single-precision)"))
  (bind (_outlocation _outrotation) (`self.GetActorEyesViewPoint` (`self.K2_GetPawn`)))
  (bind (_basevectorlocationout _caneendvector) (`self.FindCaneEnd` _outlocation _outrotation (`self.CaneLength`)))
  (`KismetSystemLibrary.DrawDebugLine` _basevectorlocationout _caneendvector (struct :`R` 1.0 :`A` 1.0) 0.0 (`self.CaneThickness`)))

(fn `FindCaneEnd`
  (params (BaseVectorLocationIn :type "Vector Structure") (ActorViewRotation :type "Rotator Structure") (CaneLength :type "Float (double-precision)"))
  (returns (BaseVectorLocationOut :type "Vector Structure") (CaneEndVector :type "Vector Structure") (RotationXVector :type "Vector Structure") (EndUnitVector :type "Vector Structure"))
  (bind _returnvalue (`KismetMathLibrary.Conv_RotatorToVector` ActorViewRotation))
  (return BaseVectorLocationIn (+ BaseVectorLocationIn (* _returnvalue CaneLength)) _returnvalue (+ BaseVectorLocationIn _returnvalue)))

(fn `UserConstructionScript`)