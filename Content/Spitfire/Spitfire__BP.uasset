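; Player-controlled Spitfire aircraft Blueprint that routes flight input to its control functions and sets up the throttle HUD.
; On BeginPlay it initializes the SpitfireEngine and adds a ThrottleDisplay widget to the viewport.
; Pitch, yaw, roll and throttle axes, plus kill-engine and center-controls actions, pass straight to flight functions defined outside these graphs.
; Releasing Tab toggles both cameras' active state to switch between the cockpit and main views.
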(event `Key|Tab`
  (params (Key :type "Key Structure"))
  (:`Released`
    (`ActorComponent.ToggleActive` (`self.CockpitCamera`))
    (`ActorComponent.ToggleActive` (`self.Camera`))))

(event `self.ReceiveBeginPlay`
  (`self.Initialize` (`self.SpitfireEngine`))
  (bind _returnvalue (`|CreateWidget` "/Game/Blueprints/ThrottleDisplay.ThrottleDisplay_C"))
  (`UserWidget.AddToViewport` _returnvalue 0))

(event `InputAxis|ThrottleUp`
  (params (AxisValue :type "Float (single-precision)"))
  (`self.SetThrottle` AxisValue))

(event `InputAxis|PitchUp`
  (params (AxisValue :type "Float (single-precision)"))
  (`self.PitchUp` AxisValue))

(event `InputAction|KillEngine`
  (params (Key :type "Key Structure"))
  (:`Released`
    (`self.KillThrottle`)))

(event `InputAxis|YawRight`
  (params (AxisValue :type "Float (single-precision)"))
  (`self.YawRight` AxisValue))

(event `InputAction|CenterControls`
  (params (Key :type "Key Structure"))
  (:`Released`
    (`self.CenterControls`)))

(event `InputAxis|RollRight`
  (params (AxisValue :type "Float (single-precision)"))
  (`self.RollRight` AxisValue))

(fn `UserConstructionScript`)