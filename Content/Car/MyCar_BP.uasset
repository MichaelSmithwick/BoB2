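; MyCar_BP is a player-driven vehicle Blueprint with switchable camera views.
; Forward and Right input axes feed throttle and steering directly into the VehicleMovement component.
; Releasing each of four camera actions toggles the main Camera along with a left, right, top or driver view camera, with no check on which other view is active.
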(event `InputAction|ToggleCameraLeft`
  (params (Key :type "Key Structure"))
  ;[1 1 1] Swap Cameras
  (:`Released`
    (`ActorComponent.ToggleActive` (`self.Camera`))
    (`ActorComponent.ToggleActive` (`self.LeftSideView`))))

(event `InputAction|ToggleCameraRight`
  (params (Key :type "Key Structure"))
  ;[1 1 1] Swap Cameras
  (:`Released`
    (`ActorComponent.ToggleActive` (`self.Camera`))
    (`ActorComponent.ToggleActive` (`self.RightSideVIew`))))

(event `InputAction|ToggleCameraTop`
  (params (Key :type "Key Structure"))
  ;[1 1 1] Swap Cameras
  (:`Released`
    (`ActorComponent.ToggleActive` (`self.Camera`))
    (`ActorComponent.ToggleActive` (`self.TopCamera`))))

(event `InputAction|DriversCamera`
  (params (Key :type "Key Structure"))
  ;[1 1 1] Swap Cameras
  (:`Released`
    (`ActorComponent.ToggleActive` (`self.Camera`))
    (`ActorComponent.ToggleActive` (`self.DriversCamera`))))

(event `InputAxis|Forward`
  (params (AxisValue :type "Float (single-precision)"))
  ;[1 1 1] Movement and Direction
  (`WheeledVehicleMovementComponent.SetThrottleInput` (`self.VehicleMovement`) AxisValue))

(event `InputAxis|Right`
  (params (AxisValue :type "Float (single-precision)"))
  ;[1 1 1] Movement and Direction
  (`WheeledVehicleMovementComponent.SetSteeringInput` (`self.VehicleMovement`) AxisValue))

(fn `UserConstructionScript`)